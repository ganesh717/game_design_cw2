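; Base first-person projectile Blueprint that plays a fire sound on spawn and knocks physics-simulating CubeTarget_BP actors.
; The construction script overrides the projectile component's velocity using a normalized launch direction, scaled by power and rotated.
; Valid hits call a separate HitTarget event, whose default behaviour applies a velocity-based impulse at the hit point and destroys the projectile after a delay.
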(event `self.ReceiveBeginPlay`
  ;[1 1 1] Default fire sound
  (`GameplayStatics.PlaySoundAtLocation` "/Game/FirstPerson/Audio/FirstPersonTemplateWeaponFire02.FirstPersonTemplateWeaponFire02" (`self.K2_GetActorLocation`) (struct) 1.0 1.0 0.0 null null null) ; Play firing sound
)

(event `self.ReceiveHit`
  (params (MyComp :type "PrimitiveComponent Object Reference") (Other :type "Actor Object Reference") (OtherComp :type "PrimitiveComponent Object Reference") (bSelfMoved :type Boolean) (HitLocation :type "Vector Structure") (HitNormal :type "Vector Structure") (NormalImpulse :type "Vector Structure") (Hit :type "HitResult Structure (by ref)"))
  ;[1 1 1] Is this a valid physics target, if so call hit Event
  (bind _ascube_target_bp (cast `/Game/CubeTarget_BP` Other))
  (if (`SceneComponent.IsSimulatingPhysics` (`StaticMeshActor.StaticMeshComponent` _ascube_target_bp) "None")
    (`self.HitTarget` _ascube_target_bp HitLocation)))

(event `HitTarget`
  (params (Target :type "/Game/CubeTarget_BP Object Reference") (HitLocation :type "Vector Structure"))
  ;[1 1 1] Default Hitting object behaviour
  (`PrimitiveComponent.AddImpulseAtLocation` (`StaticMeshActor.StaticMeshComponent` Target) (* (`self.GetVelocity`) 200.0) HitLocation "None")
  (`KismetSystemLibrary.Delay` 5.0)
  (`self.K2_DestroyActor`))

(fn `UserConstructionScript`
  ;[1 1 1] Construction is run before Begin, it also runs in editor
  ;[1 1 1] Override projectile Velocity, needs to have InitialVelocity set at 0 in Viewport to work
  (set `MovementComponent.Velocity` (`KismetMathLibrary.GreaterGreater_VectorRotator` (* (`KismetMathLibrary.Normal` (`self.LaunchDirection`)) (`self.Power`)) (`self.Rotation`)) (`self.Projectile`)))